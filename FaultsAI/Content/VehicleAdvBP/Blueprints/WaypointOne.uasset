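; WaypointOne is a track trigger that makes a Buggy of one team slide through a turn, once its sphere is entered.
; On overlap, a Buggy not yet flagged FirstToGo has its MistakeSteering lowered randomly, full AutoThotle set, and handbrake pulsed.
; On exit, it adds a separate random amount back to steering, so the offset may persist, then restores normal throttle and sets FirstToGo to prevent repeats.
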(event `self.Sphere.OnComponentBeginOverlap`
  (params (OverlappedComponent :type "PrimitiveComponent Object Reference") (OtherActor :type "Actor Object Reference") (OtherComp :type "PrimitiveComponent Object Reference") (OtherBodyIndex :type Integer) (bFromSweep :type Boolean) (SweepResult :type "HitResult Structure (by ref)"))
  (bind _asbuggy (cast `/Game/VehicleAdvBP/Blueprints/Buggy` OtherActor))
  (bind _output_get (set `self.BuggyRef` _asbuggy))
  (if (`|EnumEquality` (`/Game/VehicleAdvBP/Blueprints/Buggy.TeamEnumRef` _output_get) "NewEnumerator0")
    (if (not (`/Game/VehicleAdvBP/Blueprints/Buggy.FirstToGo` _output_get))
      (`self.SlideOnTurn`))))

(event `self.Sphere.OnComponentEndOverlap`
  (params (OverlappedComponent :type "PrimitiveComponent Object Reference") (OtherActor :type "Actor Object Reference") (OtherComp :type "PrimitiveComponent Object Reference") (OtherBodyIndex :type Integer))
  (bind _asbuggy (cast `/Game/VehicleAdvBP/Blueprints/Buggy` OtherActor))
  (bind _output_get (set `self.BuggyRef` _asbuggy))
  (if (`|EnumEquality` (`/Game/VehicleAdvBP/Blueprints/Buggy.TeamEnumRef` _output_get) "NewEnumerator0")
    (if (not (`/Game/VehicleAdvBP/Blueprints/Buggy.FirstToGo` _output_get))
      (`self.ResetSteering`))))

(fn `ResetSteering`
  (bind _buggyref (`self.BuggyRef`))
  (set `/Game/VehicleAdvBP/Blueprints/Buggy.MistakeSteering` (+ (`/Game/VehicleAdvBP/Blueprints/Buggy.MistakeSteering` (`self.BuggyRef`)) (`self.RandomFloat`)) _buggyref)
  (`/Game/VehicleAdvBP/Blueprints/Buggy.NormalAutoThrottle` _buggyref)
  (set `/Game/VehicleAdvBP/Blueprints/Buggy.FirstToGo` true (`self.BuggyRef`)))

(fn `SlideOnTurn`
  (bind _buggyref (`self.BuggyRef`))
  (set `/Game/VehicleAdvBP/Blueprints/Buggy.MistakeSteering` (- (`/Game/VehicleAdvBP/Blueprints/Buggy.MistakeSteering` (`self.BuggyRef`)) (`self.RandomFloat`)) _buggyref)
  (set `/Game/VehicleAdvBP/Blueprints/Buggy.AutoThotle` 1.0 _buggyref)
  (`/Game/VehicleAdvBP/Blueprints/Buggy.Handbreak` _buggyref)
  (`/Game/VehicleAdvBP/Blueprints/Buggy.ReleaseBreak` _buggyref))

(fn `UserConstructionScript`)