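; Spline path actor that drives a referenced vehicle by feeding it a steering target and automatic throttle every tick.
; The target is the closest path point to the vehicle's location shifted along the negated local spline right vector, marked by a sphere.
; An arrow shows the nearest path point and that reversed direction.
; Throttle is on/off below a speed threshold; a speed-and-distance throttle calculation is left unconnected.
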(event `self.ReceiveTick`
  (params (DeltaSeconds :type "Float (single-precision)"))
  (bind _vehicleref (`self.VehicleRef`))
  (bind _path (`self.Path`))
  (bind _returnvalue (`self.K2_GetActorLocation` _vehicleref))
  (bind _returnvalue_2 (`KismetMathLibrary.MakeRotationFromAxes` (`SplineComponent.FindRightVectorClosestToWorldLocation` _path _returnvalue "Local")))
  (bind _output_get (set `/Game/VehicleAdvBP/Blueprints/Buggy.Steering` (`SplineComponent.FindLocationClosestToWorldLocation` _path (- _returnvalue (* (`KismetMathLibrary.GetForwardVector` _returnvalue_2) 500.0)) "World") _vehicleref))
  (`SceneComponent.K2_SetWorldLocation` (`self.Sphere`) _output_get false false)
  (`SceneComponent.K2_SetWorldLocationAndRotation` (`self.Arrow`) (`SplineComponent.FindLocationClosestToWorldLocation` _path _returnvalue "World") (`KismetMathLibrary.MakeRotator` (.roll _returnvalue_2) (.pitch _returnvalue_2) (- (.yaw _returnvalue_2) 180.0)) false false)
  (set `/Game/VehicleAdvBP/Blueprints/Buggy.AutoThotle` (`KismetMathLibrary.SelectFloat` 1.0 0.0 (< (* (`WheeledVehicleMovementComponent.GetForwardSpeed` (`WheeledVehicle.VehicleMovement` (`self.VehicleRef`))) 0.02) 20.0)) (`self.VehicleRef`)))

(fn `UserConstructionScript`)