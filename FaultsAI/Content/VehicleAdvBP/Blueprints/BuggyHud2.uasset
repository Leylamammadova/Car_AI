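; BuggyHud2 is a HUD Blueprint that draws the possessed Buggy's speed and gear on screen.
; DrawHUD casts the owning pawn to Buggy and draws only while its IsInCar0 flag is false.
; Text position and scale follow screen-size ratios computed from a 1280x720 baseline.
; The Buggy supplies both display strings, and the gear text switches color in reverse.
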(event `self.ReceiveDrawHUD`
  (params (SizeX :type Integer) (SizeY :type Integer))
  (bind _hudyratio (`self.HUDYRatio`))
  (bind _hudyratio_2 (`self.HUDYRatio`))
  ;[1 1 1] Calculate ratio from 720p
  (bind _asbuggy (cast `/Game/VehicleAdvBP/Blueprints/Buggy` (`self.GetOwningPawn`)))
  (if (not (`/Game/VehicleAdvBP/Blueprints/Buggy.IsInCar_0` _asbuggy))
    (`|ExecutionSequence`
      (:`then_0`
        (set `self.HUDXRatio` (/ (`KismetMathLibrary.Conv_IntToDouble` SizeX) 1280.0)))
      (:`then_1`
        (set `self.HUDYRatio` (/ (`KismetMathLibrary.Conv_IntToDouble` SizeY) 720.0)))
      (:`then_2`
        ;[1 1 1] Print vehicle speed
        (bind _asbuggy_2 (cast `/Game/VehicleAdvBP/Blueprints/Buggy` (`self.GetOwningPawn`)))
        (`self.DrawText` (`/Game/VehicleAdvBP/Blueprints/Buggy.Speed Display String` _asbuggy_2) (struct :`R` 1.0 :`G` 1.0 :`B` 1.0 :`A` 1.0) (* 805.0 (`self.HUDXRatio`)) (* 455.0 _hudyratio_2) "/Engine/EngineFonts/RobotoDistanceField.RobotoDistanceField" (* 1.4 _hudyratio_2))
        ;[1 1 1] Print vehicle gear
        (bind _asbuggy_3 (cast `/Game/VehicleAdvBP/Blueprints/Buggy` (`self.GetOwningPawn`)))
        (`self.DrawText` (`/Game/VehicleAdvBP/Blueprints/Buggy.Gear Display String` _asbuggy_3) (`KismetMathLibrary.SelectColor` (`/Game/VehicleAdvBP/Blueprints/Buggy.GearDisplayReverseColor` _asbuggy_3) (`/Game/VehicleAdvBP/Blueprints/Buggy.GearDisplayColor` _asbuggy_3) (`/Game/VehicleAdvBP/Blueprints/Buggy.InReverseGear` _asbuggy_3)) (* 805.0 (`self.HUDXRatio`)) (* 500.0 _hudyratio) "/Engine/EngineFonts/RobotoDistanceField.RobotoDistanceField" (* 1.4 _hudyratio)) ; If True display Current Gear
      ))))

(fn `UserConstructionScript`)